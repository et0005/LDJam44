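; PowerStations is a one-shot power station that gives the player energy on contact.
; When a ThirdPersonCharacter overlaps its Box, a DoOnce gate calls AddEnergy on that character, plays a shock sound at the Cube and starts GrowSize.
; GrowSize re-calls itself after a short delay to steadily expand EnergyBox, until the component is destroyed a few seconds after activation.
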(event `self.Box.OnComponentBeginOverlap`
  (params (OverlappedComponent :type "PrimitiveComponent Object Reference") (OtherActor :type "Actor Object Reference") (OtherComp :type "PrimitiveComponent Object Reference") (OtherBodyIndex :type Integer) (bFromSweep :type Boolean) (SweepResult :type "HitResult Structure (by ref)"))
  ;[1 1 1] Check that the tesla hasn't gone off and that the player is the one overlapping
  (bind _asthird_person_character (cast `/Game/ThirdPersonBP/Blueprints/ThirdPersonCharacter` OtherActor))
  (`/Engine/EditorBlueprintResources/StandardMacros.DoOnce` false
    (:`Completed`
      (`/Game/ThirdPersonBP/Blueprints/ThirdPersonCharacter.AddEnergy` _asthird_person_character)
      (`GameplayStatics.PlaySoundAtLocation` "/Game/Sound/ShockSound.ShockSound" (`SceneComponent.K2_GetComponentLocation` (`self.Cube`)) (struct) 1.0 1.0 0.0 null null null)
      (`self.GrowSize`)
      (`KismetSystemLibrary.Delay` 3.5)
      (`ActorComponent.K2_DestroyComponent` (`self.EnergyBox`)))))

(event `GrowSize`
  (bind _energybox (`self.EnergyBox`))
  ;[1 1 1] Energy Box Expand
  (if (`KismetSystemLibrary.IsValid` _energybox)
    (`SceneComponent.SetWorldScale3D` _energybox (+ (`SceneComponent.K2_GetComponentScale` _energybox) 0.1))
    (`KismetSystemLibrary.Delay` 0.01)
    (`self.GrowSize`)))

(fn `UserConstructionScript`)